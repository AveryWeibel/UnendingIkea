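; BP_Quest1 is a quest in the QSys quest system that sends the player to three furniture destinations.
; CreateRootObjCollection builds an order-required BP_ObjCollect named "Ikea" as the root objective collection.
; PopObj fills that collection with three BP_ObjReach objectives in sequence, each constructed at runtime with its own destination reference and display name.
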(fn `CreateRootObjCollection`
  (returns (RootObjCollect :type "/Game/QSys/Objectives/BP_ObjCollect Object Reference"))
  (bind _returnvalue (`|GenericCreateObject` "/Game/QSys/Objectives/BP_ObjCollect.BP_ObjCollect_C" self true "Ikea"))
  (return _returnvalue))

(fn `PopObj`
  (params (RootObjCol :type "/Game/QSys/Objectives/BP_ObjCollect Object Reference"))
  (`|ExecutionSequence`
    (:`then_0`
      (bind _returnvalue (`|GenericCreateObject` "/Game/QSys/Objectives/BP_ObjReach.BP_ObjReach_C" self (`self.FurnitureTrigger`) "Stuff"))
      (`/Game/QSys/Objectives/BP_ObjCollect.AddObjective` (`local.RootObjCol`) _returnvalue))
    (:`then_1`
      (bind _returnvalue_2 (`|GenericCreateObject` "/Game/QSys/Objectives/BP_ObjReach.BP_ObjReach_C" self (`self.Furn2`) "MOAR Stuff"))
      (`/Game/QSys/Objectives/BP_ObjCollect.AddObjective` (`local.RootObjCol`) _returnvalue_2))
    (:`then_2`
      (bind _returnvalue_3 (`|GenericCreateObject` "/Game/QSys/Objectives/BP_ObjReach.BP_ObjReach_C" self (`self.Furn3`) "EVEN MORE"))
      (`/Game/QSys/Objectives/BP_ObjCollect.AddObjective` (`local.RootObjCol`) _returnvalue_3))))

(fn `UserConstructionScript`
  (`parent.UserConstructionScript`))