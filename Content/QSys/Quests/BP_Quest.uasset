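; BP_Quest is an abstract base quest Blueprint that sets up and activates a root objective collection.
; On BeginPlay it creates and stores the collection, passes it to PopObj, then calls ActiveObj on it.
; CreateRootObjCollection and PopObj are placeholders that only print abstract-call errors, leaving child quests to override them.
; A getter exposes the stored root collection.
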(event `self.ReceiveBeginPlay`
  (bind _rootobjcollect (`self.CreateRootObjCollection`))
  (bind _output_get (set `self.RootObjCollection` _rootobjcollect))
  (`self.PopObj` _output_get)
  (`/Game/QSys/Objectives/BP_Objective.ActiveObj` (`self.RootObjCollection`)))

(fn `CreateRootObjCollection`
  (returns (RootObjCollect :type "/Game/QSys/Objectives/BP_ObjCollect Object Reference"))
  (`KismetSystemLibrary.PrintString` "Error: Abstract CreateRootCollect Call" true true (struct :`R` 1.0 :`B` 0.089263 :`A` 1.0) 5.0)
  (return null))

(fn `GetRootObjCollection`
  (returns (RootObjCollection :type "/Game/QSys/Objectives/BP_ObjCollect Object Reference"))
  (return (`self.RootObjCollection`)))

(fn `PopObj`
  (params (RootObjCol :type "/Game/QSys/Objectives/BP_ObjCollect Object Reference"))
  (`KismetSystemLibrary.PrintString` "Error: Abstract PopIObj Call" true true (struct :`R` 1.0 :`B` 0.089263 :`A` 1.0) 5.0)
  (return))

(fn `UserConstructionScript`)