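; BP_ObjReach is a quest objective that completes when the player reaches a destination actor.
; On activation it calls the parent logic and binds to the Destination actor's begin-overlap event.
; When a FirstPersonCharacter overlaps it, the objective unbinds, sets IsReached and fires the completion callback with itself.
; GetComplete reports that flag.
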(event `self.ActiveObj`
  (`parent.ActiveObj`)
  (add `Actor.OnActorBeginOverlap` (`self.Destination`) (delegate `OnActorBeginOverlap_Event_0`)))

(event `OnActorBeginOverlap_Event_0`
  (params (OverlappedActor :type "Actor Object Reference") (OtherActor :type "Actor Object Reference"))
  (cast `/Game/UnrealDefaultStuff/FirstPersonBP/Blueprints/FirstPersonCharacter` OtherActor)
  (remove `Actor.OnActorBeginOverlap` (`self.Destination`) (delegate `OnActorBeginOverlap_Event_0`))
  (set `self.isReached` true)
  (`self.OnCompleted` self))

(fn `GetComplete`
  (returns (Complete :type Boolean))
  (return (`self.isReached`)))