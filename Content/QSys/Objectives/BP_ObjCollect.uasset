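; BP_ObjCollect is a composite quest objective that groups child objectives and reports complete only when all of them are complete.
; When OrderReq is set, activation starts the first incomplete child and binds its OnCompleted, which unbinds and activates the next incomplete one.
; Without OrderReq, it activates every child at once, with no completion bindings.
; AddObjective appends children to the list.
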(event `OnCompleted_Event_0` :!signature `self.OnCompleted`
  (params (Objective :type "/Game/QSys/Objectives/BP_Objective Object Reference"))
  (remove `self.OnCompleted` Objective (delegate `OnCompleted_Event_0`))
  (bind _nextobj (`self.FindNextObj` :!label _label))
  (`/Engine/EditorBlueprintResources/StandardMacros.IsValid` _nextobj
    (:`Is Valid`
      (`self.ActiveObj` _nextobj)
      (add `self.OnCompleted` _nextobj (delegate `OnCompleted_Event_0`)))))

(event `self.ActiveObj`
  (`parent.ActiveObj`)
  (if (`self.OrderReq`)
    (goto _label)
    (else
      (for _array_element (`self.Objectives`)
        (`self.ActiveObj` _array_element)))))

(fn `AddObjective`
  (params (Objective :type "/Game/QSys/Objectives/BP_Objective Object Reference"))
  (`KismetArrayLibrary.Array_Add` (`self.Objectives`) Objective))

(fn `FindNextObj`
  (returns (NextObj :type "/Game/QSys/Objectives/BP_Objective Object Reference"))
  (for _array_element (`self.Objectives`)
    (if (not (`self.GetComplete` _array_element))
      (return _array_element)))
  (return null))

(fn `GetComplete`
  (returns (Complete :type Boolean))
  (for _array_element (`self.Objectives`)
    (if (not (`self.GetComplete` _array_element))
      (return false)))
  (return true))