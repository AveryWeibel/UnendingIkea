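; Furniture-topping actor that picks a prop mesh, such as a lamp, book, pen or pen cup, on BeginPlay.
; ChooseTopping uses the set type or rolls a random enum value, then draws a random mesh from that type's array in RandomToppingTypes.
; UpdateMesh applies it to FurnitureLocation, using material slot 1 as the source for two table lamps.
; The actor's tag is set through GetNameFromString from the mesh name and printed.
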(event `self.ReceiveBeginPlay`
  (bind _topping (`self.ChooseTopping`))
  (`self.UpdateMesh` (`self.FurnitureLocation`) _topping)
  (set `self.Tags` (`|MakeArray` (`self.GetNameFromString` (`KismetSystemLibrary.GetObjectName` _topping))))
  (`KismetSystemLibrary.PrintString` (`KismetStringLibrary.Conv_NameToString` (`|GetArrayItem` (`self.Tags`))) true true (struct :`R` 1.0 :`G` 0.193061 :`B` 0.875767 :`A` 1.0)))

(fn `ChooseTopping`
  (returns (Topping :type "StaticMesh Object Reference"))
  (locals (ToppingObject :type "StaticMesh Object Reference") (FurnatureArray :type "Array of StaticMesh Object Reference"))
  (bind (_value _returnvalue) (`BlueprintMapLibrary.Map_Find` (`.ToppingTypes_7_2F3DEB3348A99124705781BF1CCEE411` (break `/Game/IkeaContent/Misc/ToppingsManager` (`self.RandomToppingTypes`))) (`self.ThisToppingType`)))
  (bind _returnvalue_2 (cast `/Game/IkeaContent/Misc/EToppingTypes` (`KismetMathLibrary.Conv_IntToByte` (`KismetMathLibrary.RandomInteger` (enumcount `/Game/IkeaContent/Misc/EToppingTypes`)))))
  (if (`|EnumEquality` (`self.ThisToppingType`) "NewEnumerator6")
    (switch `/Game/IkeaContent/Misc/EToppingTypes` _returnvalue_2
      (:`NewEnumerator4`
        (set `self.ThisToppingType` "NewEnumerator9" :!label _label))
      (:`NewEnumerator6`
        (goto _label))
      (:`NewEnumerator5`
        (set `self.ThisToppingType` _returnvalue_2 :!label _label_2))
      (:`NewEnumerator7`
        (goto _label_2))
      (:`NewEnumerator8`
        (goto _label_2))
      (:`NewEnumerator9`
        (goto _label_2)))
    (bind _output_get (set `local.ToppingObject` (`KismetArrayLibrary.Array_Random` (`.ToppingsArray_7_75CB9C4B4BB08DE88A8F5F9AB01B596C` (break `/Game/IkeaContent/Misc/ToppingsArrayStruct` _value))) :!label _label_3))
    (return _output_get)
    (elif _returnvalue
      (goto _label_3)
      (else
        (`KismetSystemLibrary.PrintString` (`KismetStringLibrary.Concat_StrStr` "[ERROR] There is no object array for furniture type " (`|GetEnumeratorNameAsString` (`self.ThisToppingType`))) true true (struct :`R` 1.0 :`G` 0.007073 :`A` 1.0))))))

(fn `UpdateMeshFunction`
  (params (`Target Mesh` :type "StaticMeshComponent Object Reference") (`New Mesh` :type "StaticMesh Object Reference"))
  (`StaticMeshComponent.SetStaticMesh` `Target Mesh` `New Mesh`)
  (`PrimitiveComponent.SetMaterial` `Target Mesh` 0 (`StaticMesh.GetMaterial` `New Mesh` 0)))

(fn `UserConstructionScript`)