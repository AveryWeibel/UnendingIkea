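; Main floor tile for the Ikea level, tracking which directions have tiles and requesting new ones from a TileManager.
; SpawnTiles forwards direction and culling to the manager's SpawnTile with a zero input tile, leaving its SpawnPosition argument unused.
; RegisterTile adds a direction to ActiveTiles, or prints a message if already present, and returns whether it was a duplicate.
; The event graph and construction script are empty.
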(fn `Register Tile`
  (params (NewTile :type "/Game/IkeaContent/Misc/EWrapDirections Enum" :default "NewEnumerator0"))
  (returns (ContainsTile :type Boolean))
  (bind _output_get (set `self.ContainsTile` (`BlueprintSetLibrary.Set_Contains` (`self.ActiveTiles`) NewTile)))
  (if _output_get
    (`KismetSystemLibrary.PrintString` (`KismetStringLibrary.Concat_StrStr` "Already contains tile in " (`|GetEnumeratorNameAsString` NewTile) "Direction"))
    (else
      (`BlueprintSetLibrary.Set_Add` (`self.ActiveTiles`) NewTile)))
  (return (`self.ContainsTile`)))

(fn `SpawnTiles`
  (params (SpawnDirection :type "/Game/IkeaContent/Misc/EWrapDirections Enum" :default "NewEnumerator0") (SpawnPosition :type "Vector Structure") (Culling :type Boolean))
  (`/Game/IkeaContent/Blueprints/TileManager.Spawn Tile` (`self.TileManager`) (0.0 0.0 0.0) SpawnDirection Culling))

(fn `UserConstructionScript`)