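; Trigger volume, placed as a child actor of an IkeaMainFloor, that extends the tiled Ikea level when the player enters it.
; The construction script caches the parent floor's location and converts WrapDirections into an array.
; On FirstPersonCharacter overlap, it calls the parent's SpawnTiles for each direction, positioned by the DirectionOffsets lookup scaled by LevelFloorSize.
; It then destroys itself, so each trigger fires only once.
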(event `self.ReceiveActorBeginOverlap`
  (params (OtherActor :type "Actor Object Reference"))
  ;[1 1 1] Foreach direction, find the offset vector and spawn an object at that location
  (if (== (`GameplayStatics.GetObjectClass` OtherActor) "/Game/UnrealDefaultStuff/FirstPersonBP/Blueprints/FirstPersonCharacter.FirstPersonCharacter_C")
    (for _array_element (`self.WrapDirectionsArray`)
      (bind _asikea_main_floor (cast `/Game/IkeaContent/Blueprints/IkeaMainFloor` (`self.GetParentActor`)))
      (`/Game/IkeaContent/Blueprints/IkeaMainFloor.SpawnTiles` _asikea_main_floor _array_element (+ (`self.ThisLevelTransform`) (* (`BlueprintMapLibrary.Map_Find` (`self.DirectionOffsets`) _array_element) (`self.LevelFloorSize`)))))
    (`self.K2_DestroyActor`)))

(fn `UserConstructionScript`
  (set `self.ThisLevelTransform` (`self.K2_GetActorLocation` (`self.GetParentActor`)))
  (bind _result (`BlueprintSetLibrary.Set_ToArray` (`self.WrapDirections`)))
  (set `self.WrapDirectionsArray` _result))