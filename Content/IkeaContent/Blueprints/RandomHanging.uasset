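; RandomHanging shows a random furniture mesh, chosen when play begins.
; ChooseFurniture picks from the RandomFurnitureTypes array for its type; RandomType rolls an enum value first, and a fixed type lacking an array prints an error.
; The mesh and its first material go onto FurnitureLocation.
; The actor's tags become a name derived from the mesh's object name, which is printed before CallGroupFurniture runs.
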(event `self.ReceiveBeginPlay`
  (bind _furniture (`self.ChooseFurniture`))
  (`self.UpdateMesh` (`self.FurnitureLocation`) _furniture)
  (set `self.Tags` (`|MakeArray` (`self.GetNameFromString` (`KismetSystemLibrary.GetObjectName` _furniture))))
  (`KismetSystemLibrary.PrintString` (`KismetStringLibrary.Conv_NameToString` (`|GetArrayItem` (`self.Tags`))) true true (struct :`R` 1.0 :`G` 0.193061 :`B` 0.875767 :`A` 1.0))
  (`self.GroupFurniture`))

(fn `ChooseFurniture`
  (returns (Furniture :type "StaticMesh Object Reference"))
  (locals (FurnatureObject :type "StaticMesh Object Reference") (FurnatureArray :type "Array of StaticMesh Object Reference"))
  (bind (_value _returnvalue) (`BlueprintMapLibrary.Map_Find` (`.FurnitureTypes_4_2F3DEB3348A99124705781BF1CCEE411` (break `/Game/IkeaContent/Misc/FurnitureManager` (`self.RandomFurnitureTypes`))) (`self.ThisFurnitureType`)))
  (bind _returnvalue_2 (cast `/Game/IkeaContent/Misc/EFurnitureTypes` (`KismetMathLibrary.Conv_IntToByte` (`KismetMathLibrary.RandomInteger` (enumcount `/Game/IkeaContent/Misc/EFurnitureTypes`)))))
  (if (`|EnumEquality` (`self.ThisFurnitureType`) "NewEnumerator6")
    (switch `/Game/IkeaContent/Misc/EFurnitureTypes` _returnvalue_2
      (:`NewEnumerator4`
        (set `self.ThisFurnitureType` "NewEnumerator0" :!label _label))
      (:`NewEnumerator6`
        (goto _label))
      (:`NewEnumerator0`
        (set `self.ThisFurnitureType` _returnvalue_2 :!label _label_2))
      (:`NewEnumerator1`
        (goto _label_2))
      (:`NewEnumerator2`
        (goto _label_2))
      (:`NewEnumerator3`
        (goto _label_2))
      (:`NewEnumerator5`
        (goto _label_2)))
    (bind _output_get (set `local.FurnatureObject` (`KismetArrayLibrary.Array_Random` (`.FurnitureArray_5_75CB9C4B4BB08DE88A8F5F9AB01B596C` (break `/Game/IkeaContent/Misc/FurnitureArrayStruct` _value))) :!label _label_3))
    (return _output_get)
    (elif _returnvalue
      (goto _label_3)
      (else
        (`KismetSystemLibrary.PrintString` (`KismetStringLibrary.Concat_StrStr` "[ERROR] There is no object array for furniture type " (`|GetEnumeratorNameAsString` (`self.ThisFurnitureType`))) true true (struct :`R` 1.0 :`G` 0.007073 :`A` 1.0))))))

(fn `UpdateMeshFunction`
  (params (`Target Mesh` :type "StaticMeshComponent Object Reference") (`New Mesh` :type "StaticMesh Object Reference"))
  (`StaticMeshComponent.SetStaticMesh` `Target Mesh` `New Mesh`)
  (`PrimitiveComponent.SetMaterial` `Target Mesh` 0 (`StaticMesh.GetMaterial` `New Mesh` 0)))

(fn `UserConstructionScript`)